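; BP_MainGate is an environment gate actor whose two static meshes switch between blocking and passable.
; Every Tick, a sequence checks the Triggered and Open booleans independently, with Triggered controlling Staticmesh1 and Open controlling Staticmesh2.
; A true flag disables that mesh's collision, while a false one restores query and physics collision.
; Nothing in this Blueprint sets either flag or changes mesh visibility or position.
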(event `self.ReceiveTick`
  (params (DeltaSeconds :type "Float (single-precision)"))
  (`|ExecutionSequence`
    (:`then_0`
      (if (`self.triggered`)
        (`PrimitiveComponent.SetCollisionEnabled` (`self.staticmesh1`) "NoCollision")
        (else
          (`PrimitiveComponent.SetCollisionEnabled` (`self.staticmesh1`) "QueryAndPhysics"))))
    (:`then_1`
      (if (`self.open`)
        (`PrimitiveComponent.SetCollisionEnabled` (`self.staticmesh2`) "NoCollision")
        (else
          (`PrimitiveComponent.SetCollisionEnabled` (`self.staticmesh2`) "QueryAndPhysics"))))))

(fn `UserConstructionScript`)